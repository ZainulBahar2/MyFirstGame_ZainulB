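; Jaelangkung NPC that shows dialog and triggers a key-item event on DoorTalk when the conversation ends.
; Once LockInteract sets IsLocked, inner and outer overlap spheres toggle billboard prompt icons for the player.
; Each Talk call advances through the Dialog array in a W_Dialog widget.
; After the last line it removes the widget, then a DoOnce calls JKeyItem and destroys both spheres.
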(event OnComponentBeginOverlap(OSphere1)
  (params (OverlappedComponent :type Primitive%20Component%20Object%20Reference) (OtherActor :type Actor%20Object%20Reference) (OtherComp :type Primitive%20Component%20Object%20Reference) (OtherBodyIndex :type Integer) (bFromSweep :type Boolean) (SweepResult :type Hit%20Result%20Structure%20%28by%20ref%29))
  ;[1 1 1] Comment
  (if (Variables|Default|GetIsLocked)
    (if (== OtherActor (Game|GetPlayerCharacter 0))
      (Rendering|SetVisibility (Variables|Components|GetOuterrIconBillboard1) true false))))

(event OnComponentEndOverlap(OSphere1)
  (params (OverlappedComponent :type Primitive%20Component%20Object%20Reference) (OtherActor :type Actor%20Object%20Reference) (OtherComp :type Primitive%20Component%20Object%20Reference) (OtherBodyIndex :type Integer))
  ;[1 1 1] Comment
  (if (== OtherActor (Game|GetPlayerCharacter 0))
    (Rendering|SetVisibility (Variables|Components|GetOuterrIconBillboard1) false false)))

(event OnComponentBeginOverlap(iSphere)
  (params (OverlappedComponent :type Primitive%20Component%20Object%20Reference) (OtherActor :type Actor%20Object%20Reference) (OtherComp :type Primitive%20Component%20Object%20Reference) (OtherBodyIndex :type Integer) (bFromSweep :type Boolean) (SweepResult :type Hit%20Result%20Structure%20%28by%20ref%29))
  ;[1 1 1] Comment
  (if (Variables|Default|GetIsLocked)
    (if (== OtherActor (Game|GetPlayerCharacter 0))
      (Rendering|SetVisibility (Variables|Components|GetInnerIconBillboard1) true false)
      (Rendering|SetVisibility (Variables|Components|GetOuterrIconBillboard1) false false))))

(event OnComponentEndOverlap(iSphere)
  (params (OverlappedComponent :type Primitive%20Component%20Object%20Reference) (OtherActor :type Actor%20Object%20Reference) (OtherComp :type Primitive%20Component%20Object%20Reference) (OtherBodyIndex :type Integer))
  ;[1 1 1] Comment
  (if (== OtherActor (Game|GetPlayerCharacter 0))
    (Rendering|SetVisibility (Variables|Components|GetInnerIconBillboard1) false false)))

(event EventLockInteract
  (params (Jaelangkung :type BP%20Jaelangkung%20NPC1%20Object%20Reference))
  (Variables|Default|SetIsLocked true))

(event EventTalk
  ;[1 1 1] Talk
  (if (Variables|Default|GetIsLocked)
    (Math|Integer|IncrementInt (Variables|Default|GetTalkIndex)
      (:%20%20
        (if (< (Variables|Default|GetTalkIndex) (Utilities|Array|Length (Variables|Default|GetDialog)))
          (Variables|Default|GetUI
            (:then
              _)
            (:else
              (bind _returnvalue (UserInterface|CreateWidget "/Game/Material/Dialog/W_Dialog.W_Dialog_C" (Game|GetPlayerController 0)))
              (bind _output_get (Variables|Default|SetUI _returnvalue))
              (UserInterface|Viewport|AddtoViewport _output_get 0)))
          (Rendering|Components|TextRender|SetText (Variables|/Game/Material/Dialog/W_Dialog.W_Dialog_C|GetTalkText (Variables|Default|GetUI)) (Utilities|Text|ToText(String) (Utilities|Array|Get(acopy) (Variables|Default|GetDialog) (Variables|Default|GetTalkIndex))))
          (else
            (Widget|RemovefromParent (Variables|Default|GetUI))
            (Utilities|FlowControl|DoOnce false
              (:Completed
                (Default|JKeyItem (Variables|Default|GetDoor%20Talk))
                (Components|DestroyComponent (Variables|Components|GetiSphere))))))))))

(fn ConstructionScript)