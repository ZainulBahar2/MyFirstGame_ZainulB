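; Interior door Blueprint that the player swings open and shut through Interact, with billboards shown at nearby trigger boxes.
; A FlipFlop plays or reverses a timeline that lerps the door's yaw through a quarter turn, adding audio each time.
; Interaction and showing billboards both require IsLocked to be true, despite its name.
; Box1 and Box4 also hide Billboard and Billboard2; Box3's end overlap does nothing.
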(event OnComponentBeginOverlap(Box2)
  (params (OverlappedComponent :type Primitive%20Component%20Object%20Reference) (OtherActor :type Actor%20Object%20Reference) (OtherComp :type Primitive%20Component%20Object%20Reference) (OtherBodyIndex :type Integer) (bFromSweep :type Boolean) (SweepResult :type Hit%20Result%20Structure%20%28by%20ref%29))
  ;[1 1 1] Comment
  (if (Variables|Default|GetIsLocked)
    (if (== OtherActor (Game|GetPlayerCharacter 0))
      (Rendering|SetVisibility (Variables|Default|GetBillboard) true false))))

(event OnComponentEndOverlap(Box2)
  (params (OverlappedComponent :type Primitive%20Component%20Object%20Reference) (OtherActor :type Actor%20Object%20Reference) (OtherComp :type Primitive%20Component%20Object%20Reference) (OtherBodyIndex :type Integer))
  ;[1 1 1] Comment
  (if (== OtherActor (Game|GetPlayerCharacter 0))
    (Rendering|SetVisibility (Variables|Default|GetBillboard) false false)))

(event OnComponentBeginOverlap(Box3)
  (params (OverlappedComponent :type Primitive%20Component%20Object%20Reference) (OtherActor :type Actor%20Object%20Reference) (OtherComp :type Primitive%20Component%20Object%20Reference) (OtherBodyIndex :type Integer) (bFromSweep :type Boolean) (SweepResult :type Hit%20Result%20Structure%20%28by%20ref%29))
  ;[1 1 1] Comment
  (if (Variables|Default|GetIsLocked)
    (if (== OtherActor (Game|GetPlayerCharacter 0))
      (Rendering|SetVisibility (Variables|Default|GetBillboard2) true false))))

(event OnComponentEndOverlap(Box3)
  (params (OverlappedComponent :type Primitive%20Component%20Object%20Reference) (OtherActor :type Actor%20Object%20Reference) (OtherComp :type Primitive%20Component%20Object%20Reference) (OtherBodyIndex :type Integer))
  ;[1 1 1] Comment
)

(event OnComponentBeginOverlap(Box1)
  (params (OverlappedComponent :type Primitive%20Component%20Object%20Reference) (OtherActor :type Actor%20Object%20Reference) (OtherComp :type Primitive%20Component%20Object%20Reference) (OtherBodyIndex :type Integer) (bFromSweep :type Boolean) (SweepResult :type Hit%20Result%20Structure%20%28by%20ref%29))
  ;[1 1 1] Comment
  (if (Variables|Default|GetIsLocked)
    (if (== OtherActor (Game|GetPlayerCharacter 0))
      (Rendering|SetVisibility (Variables|Default|GetBillboard3) true false)
      (Rendering|SetVisibility (Variables|Default|GetBillboard) false false))))

(event OnComponentEndOverlap(Box1)
  (params (OverlappedComponent :type Primitive%20Component%20Object%20Reference) (OtherActor :type Actor%20Object%20Reference) (OtherComp :type Primitive%20Component%20Object%20Reference) (OtherBodyIndex :type Integer))
  ;[1 1 1] Comment
  (if (== OtherActor (Game|GetPlayerCharacter 0))
    (Rendering|SetVisibility (Variables|Default|GetBillboard3) false false)))

(event OnComponentBeginOverlap(Box4)
  (params (OverlappedComponent :type Primitive%20Component%20Object%20Reference) (OtherActor :type Actor%20Object%20Reference) (OtherComp :type Primitive%20Component%20Object%20Reference) (OtherBodyIndex :type Integer) (bFromSweep :type Boolean) (SweepResult :type Hit%20Result%20Structure%20%28by%20ref%29))
  ;[1 1 1] Comment
  (if (Variables|Default|GetIsLocked)
    (if (== OtherActor (Game|GetPlayerCharacter 0))
      (Rendering|SetVisibility (Variables|Default|GetBillboard1) true false)
      (Rendering|SetVisibility (Variables|Default|GetBillboard) false false))))

(event OnComponentEndOverlap(Box4)
  (params (OverlappedComponent :type Primitive%20Component%20Object%20Reference) (OtherActor :type Actor%20Object%20Reference) (OtherComp :type Primitive%20Component%20Object%20Reference) (OtherBodyIndex :type Integer))
  ;[1 1 1] Comment
  (if (== OtherActor (Game|GetPlayerCharacter 0))
    (Rendering|SetVisibility (Variables|Default|GetBillboard1) false false)))

(event EventInteract
  (params (Character :type BP%20Base%20MC%20Char%20Object%20Reference))
  ;[1 1 1] Comment
  (if (Variables|Default|GetIsLocked)
    (Utilities|FlowControl|FlipFlop
      (:A
        (AddComponent|AddAudioComponent false)
        (bind _pintu (Timeline|TL_Pintu Play)
          (:Update
            (Transformation|SetWorldRotation (Variables|Default|GetPintuIndoor) (Math|Rotator|MakeRotator 0.0 0.0 (Math|Float|Lerp 0.0 9e+01 _pintu)) false false))))
      (:B
        (AddComponent|AddAudioComponent false)
        (Timeline|TL_Pintu Reverse)))))

(fn ConstructionScript)