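; Interactable double door Blueprint that swings its two leaves, PintuKanan (right) and PintuKiri (left), open and closed.
; Each Interact event toggles a FlipFlop that plays or reverses two timelines together, one per leaf.
; Their Pintu tracks drive Lerps between fixed, mirrored yaw angles a quarter turn apart.
; The angles are set as absolute world rotations, so the swing ignores the placed actor's orientation.
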(event EventInteract
  (params (Location :type Vector :default "0, 0, 0"))
  (Utilities|FlowControl|FlipFlop
    (:A
      (Utilities|FlowControl|Sequence
        (:then_0
          (bind _pintu (Timeline|Timeline Play)
            (:Update
              (Transformation|SetWorldRotation (Variables|Default|GetPintu%20Kanan) (Math|Rotator|MakeRotator 0.0 0.0 (Math|Float|Lerp 9e+01 1.8e+02 _pintu)) false false))))
        (:then_1
          (bind _pintu_2 (Timeline|TL_Pintu Play)
            (:Update
              (Transformation|SetWorldRotation (Variables|Default|GetPintuKiri) (Math|Rotator|MakeRotator 0.0 0.0 (Math|Float|Lerp -9e+01 -1.8e+02 _pintu_2)) false false))))))
    (:B
      (Utilities|FlowControl|Sequence
        (:then_0
          (Timeline|Timeline Reverse))
        (:then_1
          (Timeline|TL_Pintu Reverse))))))

(fn ConstructionScript)