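; Interior push door that the player toggles open and closed, with a timeline rotating its yaw and audio on each swing.
; Interaction and icons require both IsLocked and Talk, which PickupKeyItem and JKeyItem set true, so IsLocked effectively means unlocked.
; Overlap boxes show outer and inner icon billboards, with inner ones hiding outer ones.
; ItemTrigger reverses the door and clears Talk once; its counter self-comparison always passes.
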(event OnComponentEndOverlap(WIBox2)
  (params (OverlappedComponent :type Primitive%20Component%20Object%20Reference) (OtherActor :type Actor%20Object%20Reference) (OtherComp :type Primitive%20Component%20Object%20Reference) (OtherBodyIndex :type Integer))
  ;[1 1 1] Inner Billboard
  (if (== (Game|GetPlayerCharacter 0) OtherActor)
    (Rendering|SetVisibility (Variables|Default|GetInnerIconBillboard) false false)))

(event OnComponentBeginOverlap(WBox)
  (params (OverlappedComponent :type Primitive%20Component%20Object%20Reference) (OtherActor :type Actor%20Object%20Reference) (OtherComp :type Primitive%20Component%20Object%20Reference) (OtherBodyIndex :type Integer) (bFromSweep :type Boolean) (SweepResult :type Hit%20Result%20Structure%20%28by%20ref%29))
  ;[1 1 1] Billboard
  (if (Variables|Default|GetIsLocked)
    (if (Variables|Default|GetTalk?)
      (if (== OtherActor (Game|GetPlayerCharacter 0))
        (Rendering|SetVisibility (Variables|Default|GetOuterrIconBillboard1) true false)))))

(event OnComponentEndOverlap(WBox)
  (params (OverlappedComponent :type Primitive%20Component%20Object%20Reference) (OtherActor :type Actor%20Object%20Reference) (OtherComp :type Primitive%20Component%20Object%20Reference) (OtherBodyIndex :type Integer))
  ;[1 1 1] Billboard
  (if (== OtherActor (Game|GetPlayerCharacter 0))
    (Rendering|SetVisibility (Variables|Default|GetOuterrIconBillboard1) false false)))

(event OnComponentBeginOverlap(WBox1)
  (params (OverlappedComponent :type Primitive%20Component%20Object%20Reference) (OtherActor :type Actor%20Object%20Reference) (OtherComp :type Primitive%20Component%20Object%20Reference) (OtherBodyIndex :type Integer) (bFromSweep :type Boolean) (SweepResult :type Hit%20Result%20Structure%20%28by%20ref%29))
  ;[1 1 1] Billboard
  (if (Variables|Default|GetIsLocked)
    (if (Variables|Default|GetTalk?)
      (if (== OtherActor (Game|GetPlayerCharacter 0))
        (Rendering|SetVisibility (Variables|Default|GetOuterrIconBillboard) true false)))))

(event OnComponentEndOverlap(WBox1)
  (params (OverlappedComponent :type Primitive%20Component%20Object%20Reference) (OtherActor :type Actor%20Object%20Reference) (OtherComp :type Primitive%20Component%20Object%20Reference) (OtherBodyIndex :type Integer))
  ;[1 1 1] Billboard
  (if (== (Game|GetPlayerCharacter 0) OtherActor)
    (Rendering|SetVisibility (Variables|Default|GetOuterrIconBillboard) false false)))

(event OnComponentBeginOverlap(WIBox1)
  (params (OverlappedComponent :type Primitive%20Component%20Object%20Reference) (OtherActor :type Actor%20Object%20Reference) (OtherComp :type Primitive%20Component%20Object%20Reference) (OtherBodyIndex :type Integer) (bFromSweep :type Boolean) (SweepResult :type Hit%20Result%20Structure%20%28by%20ref%29))
  ;[1 1 1] Inner Billboard
  (if (Variables|Default|GetIsLocked)
    (if (Variables|Default|GetTalk?)
      (if (== OtherActor (Game|GetPlayerCharacter 0))
        (Rendering|SetVisibility (Variables|Default|GetInnerIconBillboard1) true false)
        (Rendering|SetVisibility (Variables|Default|GetOuterrIconBillboard1) false false)))))

(event OnComponentEndOverlap(WIBox1)
  (params (OverlappedComponent :type Primitive%20Component%20Object%20Reference) (OtherActor :type Actor%20Object%20Reference) (OtherComp :type Primitive%20Component%20Object%20Reference) (OtherBodyIndex :type Integer))
  ;[1 1 1] Inner Billboard
  (if (== (Game|GetPlayerCharacter 0) OtherActor)
    (Rendering|SetVisibility (Variables|Default|GetInnerIconBillboard1) false false)))

(event OnComponentBeginOverlap(WIBox2)
  (params (OverlappedComponent :type Primitive%20Component%20Object%20Reference) (OtherActor :type Actor%20Object%20Reference) (OtherComp :type Primitive%20Component%20Object%20Reference) (OtherBodyIndex :type Integer) (bFromSweep :type Boolean) (SweepResult :type Hit%20Result%20Structure%20%28by%20ref%29))
  ;[1 1 1] Inner Billboard
  (if (Variables|Default|GetIsLocked)
    (if (Variables|Default|GetTalk?)
      (if (== OtherActor (Game|GetPlayerCharacter 0))
        (Rendering|SetVisibility (Variables|Default|GetInnerIconBillboard) true false)
        (Rendering|SetVisibility (Variables|Default|GetOuterrIconBillboard) false false)))))

(event Custom|ItemTrigger
  (Math|Integer|IncrementInt (Variables|Default|GetItemTrigger1)
    (:%20%20
      (if (== (Variables|Default|GetItemTrigger1) (Variables|Default|GetItemTrigger1))
        (Utilities|FlowControl|Sequence
          (:then_0
            ;[1 1 1] Interaksi Pintu
            (AddComponent|AddAudioComponent false)
            (bind _pintu (Timeline|TL_Pintu Reverse)
              (:Update
                (Transformation|SetWorldRotation (Variables|Default|GetPintuIndoor) (Math|Rotator|MakeRotator 0.0 0.0 (Math|Float|Lerp 0.0 -9e+01 _pintu)) false false))))
          (:then_1
            (Utilities|FlowControl|DoOnce false
              (:Completed
                (Variables|Default|SetTalk? false)))))))))

(event EventPickupKeyItem
  (params (DoubleDoor :type BP%20FP%20Double%20Door%20Object%20Reference))
  (Variables|Default|SetIsLocked true))

(event EventJKeyItem
  (params (Talk%20Interact :type BP%20Jaelangkung%20NPC1%20Object%20Reference))
  (Variables|Default|SetTalk? true))

(event EventInteract
  (params (Character :type BP%20Base%20MC%20Char%20Object%20Reference))
  ;[1 1 1] Interaksi Pintu
  (if (Variables|Default|GetIsLocked)
    (if (Variables|Default|GetTalk?)
      (Utilities|FlowControl|FlipFlop
        (:A
          (AddComponent|AddAudioComponent false)
          (bind _pintu (Timeline|TL_Pintu Play)
            (:Update
              (Transformation|SetWorldRotation (Variables|Default|GetPintuIndoor) (Math|Rotator|MakeRotator 0.0 0.0 (Math|Float|Lerp 0.0 -9e+01 _pintu)) false false))))
        (:B
          (AddComponent|AddAudioComponent false)
          (Timeline|TL_Pintu Reverse))))))

(fn ConstructionScript)