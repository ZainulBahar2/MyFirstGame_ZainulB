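; Inspection actor that shows an item mesh with a name and description widget, taking input from the character during viewing.
; A SceneCaptureComponent2D views the mesh: left-drag rotates it, the mouse wheel zooms by clamped FOV, and right-click restores the stored rotation and default FOV.
; IA_Interact returns input to the character, removes the widget, and destroys this actor, not the stored BaseItem, if the item is pickupable.
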(event Custom|SetItemRotation
  (params (Rotator :type Rotator))
  (bind _inspect_item (Variables|Default|GetInspect%20Item))
  (bind _returnvalue (Transformation|GetWorldTransform _inspect_item))
  ;[1 1 1] Set Item Rotation and scale
  (Variables|Default|SetRotator Rotator)
  (Transformation|SetWorldTransform _inspect_item (Math|Transform|MakeTransform (.location _returnvalue) Rotator (.scale _returnvalue)) false false))

(event Custom|Set%20Item%20Scale
  (params (Inspect%20Scale :type Vector))
  (bind _inspect_item (Variables|Default|GetInspect%20Item))
  (bind _returnvalue (Transformation|GetWorldTransform _inspect_item))
  ;[1 1 1] Set Item Rotation and scale
  (Transformation|SetWorldTransform _inspect_item (Math|Transform|MakeTransform (.location _returnvalue) (.rotation _returnvalue) Inspect%20Scale) false false))

(event Input|EnhancedActionEvents|EnhancedInputActionIA_Interact
  (params (ActionValue :type Boolean) (ElapsedSeconds :type Float%20%28double-precision%29) (TriggeredSeconds :type Float%20%28double-precision%29) (InputAction :type Input%20Action%20Object%20Reference :default "/Game/Character_model/Control/IA_Interact.IA_Interact"))
  (bind _returnvalue (Game|GetPlayerController 0))
  (Input|DisableInput _returnvalue)
  (Input|EnableInput (Variables|Default|GetCharacter) _returnvalue)
  (Utilities|IsValid (Variables|Default|GetWBP_Inspect)
    (:Is%20Valid
      (Widget|RemovefromParent (Variables|Default|GetWBP_Inspect))
      (Variables|Default|SetWBP_Inspect 0)
      (if (Variables|Default|GetIsPickupAble)
        (Actor|DestroyActor)))))

(event EventInspect
  (params (Character :type BP%20Base%20MC%20Char%20Object%20Reference) (InspectedItem :type Static%20Mesh%20Object%20Reference) (ItemName :type Text) (Description :type Text) (BaseItem :type Actor%20Object%20Reference) (IsPickupAble :type Boolean))
  (bind _returnvalue (Game|GetPlayerController 0))
  (bind _output_get (Variables|Default|SetIsPickupAble IsPickupAble))
  (if _output_get
    (Variables|Default|SetBase%20Item BaseItem))
  (Variables|Default|SetCharacter Character)
  (Components|StaticMesh|SetStaticMesh (Variables|Default|GetInspect%20Item) InspectedItem)
  (bind _returnvalue_2 (UserInterface|CreateWidget "/Game/Material/Widget/WBP_ItemIdentification.WBP_ItemIdentification_C" 0 ItemName Description))
  (bind _output_get_2 (Variables|Default|SetWBP_Inspect _returnvalue_2))
  (UserInterface|Viewport|AddtoViewport _output_get_2 0)
  (Input|DisableInput (Variables|Default|GetCharacter) _returnvalue)
  (Input|EnableInput _returnvalue))

(event Input|MouseEvents|MouseX
  (params (AxisValue :type Float%20%28single-precision%29))
  (bind _inspect_item (Variables|Default|GetInspect%20Item))
  ;[1 1 1] Rotate
  (if (Variables|Default|GetIsRotating)
    (Transformation|SetWorldRotation _inspect_item (Math|Rotator|CombineRotators (Transformation|GetWorldRotation _inspect_item) (Math|Rotator|MakeRotator 0.0 0.0 (* AxisValue -3.0))) false false)))

(event Input|MouseEvents|MouseY
  (params (AxisValue :type Float%20%28single-precision%29))
  (bind _inspect_item (Variables|Default|GetInspect%20Item))
  ;[1 1 1] Rotate
  (if (Variables|Default|GetIsRotating)
    (Transformation|SetWorldRotation _inspect_item (Math|Rotator|CombineRotators (Transformation|GetWorldRotation _inspect_item) (Math|Rotator|MakeRotator 0.0 (* AxisValue -3.0) 0.0)) false false)))

(event Input|MouseEvents|LeftMouseButton
  (params (Key :type Key%20Structure :default "None"))
  ;[1 1 1] Klik
  (:Pressed
    (Variables|Default|SetIsRotating true))
  (:Released
    (Variables|Default|SetIsRotating false)))

(event Input|MouseEvents|RightMouseButton
  (params (Key :type Key%20Structure :default "None"))
  ;[1 1 1] Klik
  (:Pressed
    (Transformation|SetWorldRotation (Variables|Default|GetInspect%20Item) (Variables|Default|GetRotator) false false)
    (Variables|/Script/Engine.SceneCaptureComponent2D|SetFOVAngle (Variables|Default|GetSceneCaptureComponent2D) 5e+01)))

(event Input|MouseEvents|MouseWheelUp
  (params (Key :type Key%20Structure :default "None"))
  (bind _scenecapturecomponent2d (Variables|Default|GetSceneCaptureComponent2D))
  ;[1 1 1] Scale
  (:Pressed
    (Variables|/Script/Engine.SceneCaptureComponent2D|SetFOVAngle _scenecapturecomponent2d (Math|Float|Clamp(Float) (- (Variables|/Script/Engine.SceneCaptureComponent2D|GetFOVAngle _scenecapturecomponent2d) 1.0) 3e+01 9e+01))))

(event Input|MouseEvents|MouseWheelDown
  (params (Key :type Key%20Structure :default "None"))
  (bind _scenecapturecomponent2d (Variables|Default|GetSceneCaptureComponent2D))
  ;[1 1 1] Scale
  (:Pressed
    (Variables|/Script/Engine.SceneCaptureComponent2D|SetFOVAngle _scenecapturecomponent2d (Math|Float|Clamp(Float) (+ (Variables|/Script/Engine.SceneCaptureComponent2D|GetFOVAngle _scenecapturecomponent2d) 1.0) 3e+01 9e+01))))

(fn ConstructionScript)