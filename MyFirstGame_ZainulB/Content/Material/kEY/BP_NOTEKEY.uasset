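; BP_NOTEKEY is an interactable key pickup that can be inspected and reports its collection to a Door.
; Two overlap spheres toggle proximity billboard icons for the player, showing the outer icon, then swapping to the inner one.
; When inspectable, Interact spawns a BP_InspectionItem at a far-off location with the key's mesh and text, calls PickupKeyItem on the Door, then immediately destroys itself.
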(event OnComponentBeginOverlap(iSphere)
  (params (OverlappedComponent :type Primitive%20Component%20Object%20Reference) (OtherActor :type Actor%20Object%20Reference) (OtherComp :type Primitive%20Component%20Object%20Reference) (OtherBodyIndex :type Integer) (bFromSweep :type Boolean) (SweepResult :type Hit%20Result%20Structure%20%28by%20ref%29))
  ;[1 1 1] Comment
  (if (== OtherActor (Game|GetPlayerCharacter 0))
    (Rendering|SetVisibility (Variables|Default|GetInnerIconBillboard1) true false)
    (Rendering|SetVisibility (Variables|Default|GetOuterrIconBillboard1) false false)))

(event OnComponentEndOverlap(iSphere)
  (params (OverlappedComponent :type Primitive%20Component%20Object%20Reference) (OtherActor :type Actor%20Object%20Reference) (OtherComp :type Primitive%20Component%20Object%20Reference) (OtherBodyIndex :type Integer))
  ;[1 1 1] Comment
  (if (== OtherActor (Game|GetPlayerCharacter 0))
    (Rendering|SetVisibility (Variables|Default|GetInnerIconBillboard1) false false)))

(event OnComponentBeginOverlap(OSphere1)
  (params (OverlappedComponent :type Primitive%20Component%20Object%20Reference) (OtherActor :type Actor%20Object%20Reference) (OtherComp :type Primitive%20Component%20Object%20Reference) (OtherBodyIndex :type Integer) (bFromSweep :type Boolean) (SweepResult :type Hit%20Result%20Structure%20%28by%20ref%29))
  ;[1 1 1] Comment
  (if (== OtherActor (Game|GetPlayerCharacter 0))
    (Rendering|SetVisibility (Variables|Default|GetOuterrIconBillboard1) true false)))

(event OnComponentEndOverlap(OSphere1)
  (params (OverlappedComponent :type Primitive%20Component%20Object%20Reference) (OtherActor :type Actor%20Object%20Reference) (OtherComp :type Primitive%20Component%20Object%20Reference) (OtherBodyIndex :type Integer))
  ;[1 1 1] Comment
  (if (== OtherActor (Game|GetPlayerCharacter 0))
    (Rendering|SetVisibility (Variables|Default|GetOuterrIconBillboard1) false false)))

(event EventInteract
  (params (Character :type BP%20Base%20MC%20Char%20Object%20Reference))
  (Variables|Default|SetCharacter Character)
  (if (Variables|Default|GetIsInspectAble)
    (bind _returnvalue (Game|SpawnActorfromClass "/Game/Material/kEY/BP_InspectionItem.BP_InspectionItem_C" (Math|Transform|MakeTransform "1000000.000000,0.000000,0.000000") "Undefined" "MultiplyWithRoot" 0 0))
    (Default|Inspect _returnvalue (Variables|Default|GetCharacter) (Variables|/Script/Engine.StaticMeshComponent|GetStaticMesh (Variables|Default|GetKey)) (Variables|Default|GetItemName) (Variables|Default|GetItemDesc) self (Variables|Default|GetIs%20Pickup%20Able))
    (Default|PickupKeyItem (Variables|Default|GetDoor))
    (Actor|DestroyActor)))

(fn ConstructionScript)