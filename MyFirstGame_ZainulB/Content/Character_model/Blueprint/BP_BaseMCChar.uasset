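; BP_BaseMCChar is the base player character, with Enhanced Input look, movement, flashlight, sprint, crouch and interaction.
; BeginPlay adds IMC_BaseMapping; input toggles flashlight visibility and crouch, while sprint changes walk speed and widens camera FOV through a timeline.
; Interaction line-traces from the camera along its view and sends InteractMessage to the hit actor.
; An area-based sphere-trace interaction and a flashlight spawn are left unconnected.
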(event Custom|CustomEvent
  ;[1 1 1] Basic Awal
)

(event Input|EnhancedActionEvents|EnhancedInputActionIA_Interact
  (params (ActionValue :type Boolean) (ElapsedSeconds :type Float%20%28double-precision%29) (TriggeredSeconds :type Float%20%28double-precision%29) (InputAction :type Input%20Action%20Object%20Reference :default "/Game/Character_model/Control/IA_Interact.IA_Interact"))
  ;[1 1 1] Interaction Area
)

(event Input|EnhancedActionEvents|EnhancedInputActionIA_Interact
  (params (ActionValue :type Boolean) (ElapsedSeconds :type Float%20%28double-precision%29) (TriggeredSeconds :type Float%20%28double-precision%29) (InputAction :type Input%20Action%20Object%20Reference :default "/Game/Character_model/Control/IA_Interact.IA_Interact"))
  (bind _camera (Variables|Default|GetCamera))
  (bind _returnvalue (Transformation|GetWorldLocation _camera))
  ;[1 1 1] Interaction Point
  (bind (_outhit _returnvalue_2) (Collision|LineTraceByChannel _returnvalue (+ _returnvalue (* (Math|Vector|GetForwardVector (Transformation|GetWorldRotation _camera)) (Variables|Default|GetJarak))) "TraceTypeQuery1" false 0 "None"))
  (if _returnvalue_2
    (Class|IInterface|Interact(Message) (.HitActor (Collision|BreakHitResult _outhit)) self)))

(event Input|EnhancedActionEvents|EnhancedInputActionIA_FL
  (params (ActionValue :type Boolean) (ElapsedSeconds :type Float%20%28double-precision%29) (TriggeredSeconds :type Float%20%28double-precision%29) (InputAction :type Input%20Action%20Object%20Reference :default "/Game/Character_model/Control/IA_FL.IA_FL"))
  (bind _spotlight (Variables|Default|GetSpotLight))
  ;[1 1 1] FlashLight
  (Variables|Default|SetFlashlight%20on? (not (Variables|Default|GetFlashlight%20on?)))
  (if (Variables|Default|GetFlashlight%20on?)
    (Rendering|SetVisibility _spotlight true false)
    (else
      (Rendering|SetVisibility _spotlight false false))))

(event Input|EnhancedActionEvents|EnhancedInputActionIA_Crouch
  (params (ActionValue :type Boolean) (ElapsedSeconds :type Float%20%28double-precision%29) (TriggeredSeconds :type Float%20%28double-precision%29) (InputAction :type Input%20Action%20Object%20Reference :default "/Game/Character_model/Control/IA_Crouch.IA_Crouch"))
  ;[1 1 1] Jongkok
  (if (Variables|Default|GetJongkok)
    (Character|Crouch)
    (Variables|Default|SetJongkok false)
    (else
      (Character|UnCrouch)
      (Variables|Default|SetJongkok true))))

(event Input|EnhancedActionEvents|EnhancedInputActionIA_MoveFoward
  (params (ActionValue :type Float%20%28double-precision%29) (ElapsedSeconds :type Float%20%28double-precision%29) (TriggeredSeconds :type Float%20%28double-precision%29) (InputAction :type Input%20Action%20Object%20Reference :default "/Game/Character_model/Control/IA_MoveFoward.IA_MoveFoward"))
  (bind _returnvalue (Pawn|GetControlRotation :!class /Script/Engine.Pawn))
  ;[1 1 1] Movement
  (Pawn|Input|AddMovementInput (Math|Vector|GetForwardVector (Math|Rotator|MakeRotator (.roll _returnvalue) 0.0 (.yaw _returnvalue))) ActionValue false))

(event Input|EnhancedActionEvents|EnhancedInputActionIA_MoveRight
  (params (ActionValue :type Float%20%28double-precision%29) (ElapsedSeconds :type Float%20%28double-precision%29) (TriggeredSeconds :type Float%20%28double-precision%29) (InputAction :type Input%20Action%20Object%20Reference :default "/Game/Character_model/Control/IA_MoveRight.IA_MoveRight"))
  ;[1 1 1] Movement
  (Pawn|Input|AddMovementInput (Math|Vector|GetRightVector (Math|Rotator|MakeRotator 0.0 0.0 (.yaw (Pawn|GetControlRotation :!class /Script/Engine.Pawn)))) ActionValue false))

(event Input|EnhancedActionEvents|EnhancedInputActionIA_Look
  (params (ActionValue :type Vector%202D%20Structure) (ElapsedSeconds :type Float%20%28double-precision%29) (TriggeredSeconds :type Float%20%28double-precision%29) (InputAction :type Input%20Action%20Object%20Reference :default "/Game/Character_model/Control/IA_Look.IA_Look"))
  ;[1 1 1] Mouse
  (Pawn|Input|AddControllerYawInput (.x ActionValue))
  (Pawn|Input|AddControllerPitchInput (.y ActionValue)))

(event Input|EnhancedActionEvents|EnhancedInputActionIA_Sprint
  (params (ActionValue :type Boolean) (ElapsedSeconds :type Float%20%28double-precision%29) (TriggeredSeconds :type Float%20%28double-precision%29) (InputAction :type Input%20Action%20Object%20Reference :default "/Game/Character_model/Control/IA_Sprint.IA_Sprint"))
  (bind _charactermovement (Variables|Character|GetCharacterMovement))
  ;[1 1 1] Sprint
  (:Triggered
    (Variables|/Script/Engine.CharacterMovementComponent|SetMaxWalkSpeed _charactermovement 4e+02)
    (bind _sprint (Timeline|TL_Sprint Play)
      (:Update
        (Camera|SetFieldOfView (Variables|Default|GetCamera) (Math|Float|Lerp 9e+01 1.1e+02 _sprint)))))
  (:Canceled
    (Variables|/Script/Engine.CharacterMovementComponent|SetMaxWalkSpeed _charactermovement 2e+02 :!label _label)
    (Timeline|TL_Sprint Reverse))
  (:Completed
    (goto _label)))

(event EventBeginPlay
  ;[1 1 1] Basic Awal
  (bind _asplayer_controller (Utilities|Casting|CastToPlayerController (Pawn|GetController)))
  (Utilities|IsValid (PlayerController|LocalPlayerSubsystems|GetEnhancedInputLocalPlayerSubsystem _asplayer_controller)
    (:Is%20Valid
      (Input|AddMappingContext (PlayerController|LocalPlayerSubsystems|GetEnhancedInputLocalPlayerSubsystem _asplayer_controller) "/Game/Character_model/Control/IMC_BaseMapping.IMC_BaseMapping" 0 "(bIgnoreAllPressedKeysUntilRelease=True,bForceImmediately=False,bNotifyUserSettings=False)"))))

(event Input|KeyboardEvents|LeftCtrl
  (params (Key :type Key%20Structure :default "None")))

(fn ConstructionScript)